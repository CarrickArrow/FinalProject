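; Music manager Blueprint that plays a list of tracks and switches which one is audible.
; On BeginPlay it creates a 2D sound for every track, starts them all together at zero volume, then raises the initial track to the music volume.
; ChangeMusicTo mutes the current track and unmutes the requested index, an instant switch with no crossfade or restart.
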(event `self.ReceiveBeginPlay`
  (bind _output (`|GetArrayItem` (`self.MusicReferences`) (`self.Indexofsong to play`)))
  (for _array_element (`self.Track_List`)
    (bind _returnvalue (`GameplayStatics.CreateSound2D` _array_element 1.0 1.0 0.0 null))
    (`KismetArrayLibrary.Array_Add` (`self.MusicReferences`) _returnvalue)
    (`AudioComponent.SetVolumeMultiplier` _returnvalue 0.0)
    (`AudioComponent.Play` _returnvalue 0.0))
  (`AudioComponent.SetVolumeMultiplier` _output (`self.MusicVol`))
  (set `self.CurrentMusic Ref` _output))

(event `ChangeMusicTo`
  (params (`index of song to play` :type Integer))
  (bind _output (`|GetArrayItem` (`self.MusicReferences`) `index of song to play`))
  (`AudioComponent.SetVolumeMultiplier` (`self.CurrentMusic Ref`) 0.0)
  (`AudioComponent.SetVolumeMultiplier` _output (`self.MusicVol`))
  (set `self.CurrentMusic Ref` _output))

(fn `UserConstructionScript`)
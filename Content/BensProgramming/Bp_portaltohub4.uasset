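; Portal actor that ends a level by showing the level 3 win screen when the ThirdPersonCharacter overlaps its capsule.
; On overlap it adds the widget, pauses the game, sets game-only input and shows the mouse cursor.
; The construction script captures the scene with a cube capture component and feeds a cube map into a dynamic material instance for the Niagara effect.
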(event `self.Capsule.OnComponentBeginOverlap`
  (params (OverlappedComponent :type "PrimitiveComponent Object Reference") (OtherActor :type "Actor Object Reference") (OtherComp :type "PrimitiveComponent Object Reference") (OtherBodyIndex :type Integer) (bFromSweep :type Boolean) (SweepResult :type "HitResult Structure (by ref)"))
  (bind _returnvalue (`GameplayStatics.GetPlayerController` 0))
  (cast `/Game/ThirdPersonBP/Blueprints/ThirdPersonCharacter` OtherActor)
  (bind _returnvalue_2 (`|CreateWidget` "/Game/UserInterface/WinScreen/Win_Screen_WidgetLvl3.Win_Screen_WidgetLvl3_C"))
  (`UserWidget.AddToViewport` _returnvalue_2 0)
  (`GameplayStatics.SetGamePaused` true)
  (`WidgetBlueprintLibrary.SetInputMode_GameOnly` _returnvalue)
  (set `PlayerController.bShowMouseCursor` true _returnvalue))

(fn `UserConstructionScript`
  (`SceneCaptureComponentCube.CaptureScene` (`self.SceneCaptureComponentCube`))
  (bind _returnvalue (`KismetMaterialLibrary.CreateDynamicMaterialInstance` (`self.MaterialInstance`)))
  (`MaterialInstanceDynamic.SetTextureParameterValue` _returnvalue "Cube map" (`self.Map`))
  (`NiagaraComponent.SetVariableMaterial` (`self.Niagara`) "mic" _returnvalue))